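; Player character for an idle clicker that runs the money economy and creates the MainActivity UI.
; BeginPlay starts Delay loops that add tiered income, paced by clock and overclock, and deduct bills and taxes, updating the money text.
; The construction script loads the "main" slot, and BeginPlay autosaves periodically until a save fails.
; SaveGame writes and returns in its first Sequence branch, so only CurrentMoney reaches the slot.
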(event Custom|restartTimers
  (bind _returnvalue (Game|GetPlayerController 0))
  (bind _returnvalue_2 (UserInterface|CreateWidget "/Game/views/mainActivity.mainActivity_C" _returnvalue))
  (bind _output_get (Variables|Default|SetmainActivityRef _returnvalue_2))
  (UserInterface|Viewport|AddtoViewport _output_get 0)
  (Variables|/Script/Engine.PlayerController|SetbShowMouseCursor _returnvalue true))

(event EventBeginPlay
  (bind _returnvalue (Game|GetPlayerController 0))
  (Utilities|FlowControl|Sequence
    (:then_0
      (Utilities|FlowControl|Delay (Math|Conversions|ToFloat(Integer) (Variables|Default|GetbillTime)) :!label _label)
      (bind _output_get (Variables|Default|SetcurrentMoney (- (Variables|Default|GetcurrentMoney) (Variables|Default|Getbill))))
      (Rendering|Components|TextRender|SetText (Variables|/Game/views/mainActivity.mainActivity_C|Gettext_moneyValue (Variables|Default|GetmainActivityRef)) (Utilities|Text|ToText(Integer) _output_get))
      (goto _label))
    (:then_1
      (Utilities|FlowControl|Delay (/ (/ (Variables|Default|GetcurrentClock) (Variables|Default|GetoverclockCount)) 1e+03) :!label _label_2)
      (bind _output_get_2 (Variables|Default|SetcurrentMoney (+ (Variables|Default|GetcurrentMoney) (+ (* (Variables|Default|Gett1Count) 2) (* (Variables|Default|Gett2Count) 5) (* (Variables|Default|Gett3Count) 10) (* (Variables|Default|Gett4Count) 13) (* (Variables|Default|Gett5Count) 17) (* (Variables|Default|Gett6Count) 75) (* (Variables|Default|Gett7Count) 109) (* (Variables|Default|Gett8Count) 256) (* (Variables|Default|Gett9Count) 573) (* (Variables|Default|Gett10Count) 1244)))))
      (Rendering|Components|TextRender|SetText (Variables|/Game/views/mainActivity.mainActivity_C|Gettext_moneyValue (Variables|Default|GetmainActivityRef)) (Utilities|Text|ToText(Integer) _output_get_2))
      (goto _label_2))
    (:then_2
      (bind _returnvalue_2 (UserInterface|CreateWidget "/Game/views/mainActivity.mainActivity_C" _returnvalue))
      (bind _output_get_3 (Variables|Default|SetmainActivityRef _returnvalue_2))
      (UserInterface|Viewport|AddtoViewport _output_get_3 0)
      (Variables|/Script/Engine.PlayerController|SetbShowMouseCursor _returnvalue true))
    (:then_3
      (Utilities|FlowControl|Delay (Math|Conversions|ToFloat(Integer) (Variables|Default|GettaxTime)) :!label _label_3)
      (bind _output_get_4 (Variables|Default|SetcurrentMoney (- (Variables|Default|GetcurrentMoney) (Variables|Default|GettaxPerTime))))
      (Rendering|Components|TextRender|SetText (Variables|/Game/views/mainActivity.mainActivity_C|Gettext_moneyValue (Variables|Default|GetmainActivityRef)) (Utilities|Text|ToText(Integer) _output_get_4))
      (goto _label_3))
    (:then_4
      (Utilities|FlowControl|Delay 2e+01)
      (bind _success (CallFunction|SaveGame))
      (if _success
        (Development|PrintString "saved" true true "(R=0.000000,G=1.000000,B=0.053974,A=1.000000)" 5.0)
        (Utilities|FlowControl|Delay 5.0 :!label _label_4)
        (bind _success_2 (CallFunction|SaveGame))
        (if _success_2
          (Development|PrintString "saved" true true "(R=0.000000,G=1.000000,B=0.053974,A=1.000000)" 5.0)
          (goto _label_4))
        (else
          (Development|PrintString "NOT saved" true true "(R=1.000000,G=0.000000,B=0.000000,A=1.000000)" 5.0))))
    (:then_5
      (Development|PrintString (Utilities|String|ToString(Integer) (Variables|Default|GetcurrentMoney))))
    (:then_6
      (Development|PrintString (Utilities|String|ToString(Integer) (Variables|Default|Gett1Count))))))

(fn ConstructionScript
  (bind _success (CallFunction|LoadGame))
  (if _success
    (Development|PrintString "loaded" true true "(R=0.000000,G=0.660000,B=1.000000,A=1.000000)" 4.0)
    (else
      (Development|PrintString "not loaded" true true "(R=0.000000,G=0.660000,B=1.000000,A=1.000000)" 4.0))))

(fn SaveGame
  (bind _returnvalue (SaveGame|CreateSaveGameObject "/Game/views/saveGameObject.saveGameObject_C"))
  (Variables|Default|SetsaveGameRef _returnvalue)
  (Utilities|FlowControl|Sequence
    (:then_0
      (Variables|/Game/views/saveGameObject.saveGameObject_C|SetcurrentMoney _returnvalue (Variables|Default|GetcurrentMoney))
      (bind _returnvalue_2 (SaveGame|SaveGametoSlot _returnvalue "main"))
      (return _returnvalue_2))
    (:then_1
      (Variables|/Game/views/saveGameObject.saveGameObject_C|SetoverclockCount _returnvalue (Variables|Default|GetoverclockCount)))
    (:then_2
      (Variables|/Game/views/saveGameObject.saveGameObject_C|SetclickIncrementBoostCount _returnvalue (Variables|Default|GetclickIncrementBoostCount)))
    (:then_3
      (Variables|/Game/views/saveGameObject.saveGameObject_C|Sett1Count _returnvalue (Variables|Default|Gett1Count)))
    (:then_4
      (Variables|/Game/views/saveGameObject.saveGameObject_C|Sett2Count _returnvalue (Variables|Default|Gett2Count)))
    (:then_5
      (Variables|/Game/views/saveGameObject.saveGameObject_C|Sett3Count _returnvalue (Variables|Default|Gett3Count)))
    (:then_6
      (Variables|/Game/views/saveGameObject.saveGameObject_C|Sett4Count _returnvalue (Variables|Default|Gett4Count)))
    (:then_7
      (Variables|/Game/views/saveGameObject.saveGameObject_C|Sett5Count _returnvalue (Variables|Default|Gett5Count)))
    (:then_8
      (Variables|/Game/views/saveGameObject.saveGameObject_C|Sett6Count _returnvalue (Variables|Default|Gett6Count)))
    (:then_9
      (Variables|/Game/views/saveGameObject.saveGameObject_C|Sett7Count _returnvalue (Variables|Default|Gett7Count)))
    (:then_10
      (Variables|/Game/views/saveGameObject.saveGameObject_C|Sett8Count _returnvalue (Variables|Default|Gett8Count)))
    (:then_11
      (Variables|/Game/views/saveGameObject.saveGameObject_C|Sett9Count _returnvalue (Variables|Default|Gett9Count)))
    (:then_12
      (Variables|/Game/views/saveGameObject.saveGameObject_C|Sett10Count _returnvalue (Variables|Default|Gett10Count)))
    (:then_13
      (Variables|Default|SetclickIncrementValue (Variables|Default|GetclickIncrementValue)))))

(fn LoadGame
  (bind _returnvalue (SaveGame|DoesSaveGameExist "main"))
  (if _returnvalue
    (bind _returnvalue_2 (SaveGame|LoadGamefromSlot "main"))
    (bind _assave_game_object (Utilities|Casting|CastTosaveGameObject _returnvalue_2))
    (Utilities|FlowControl|Sequence
      (:then_0
        (Variables|Default|SetcurrentMoney (Variables|/Game/views/saveGameObject.saveGameObject_C|GetcurrentMoney _assave_game_object)))
      (:then_1
        (Variables|Default|SetoverclockCount (Variables|/Game/views/saveGameObject.saveGameObject_C|GetoverclockCount _assave_game_object)))
      (:then_2
        (Variables|Default|SetclickIncrementBoostCount (Variables|/Game/views/saveGameObject.saveGameObject_C|GetclickIncrementBoostCount _assave_game_object)))
      (:then_3
        (Variables|Default|Sett1Count (Variables|/Game/views/saveGameObject.saveGameObject_C|Gett1Count _assave_game_object)))
      (:then_4
        (Variables|Default|Sett2Count (Variables|/Game/views/saveGameObject.saveGameObject_C|Gett2Count _assave_game_object)))
      (:then_5
        (Variables|Default|Sett3Count (Variables|/Game/views/saveGameObject.saveGameObject_C|Gett3Count _assave_game_object)))
      (:then_6
        (Variables|Default|Sett4Count (Variables|/Game/views/saveGameObject.saveGameObject_C|Gett4Count _assave_game_object)))
      (:then_7
        (Variables|Default|Sett5Count (Variables|/Game/views/saveGameObject.saveGameObject_C|Gett5Count _assave_game_object)))
      (:then_8
        (Variables|Default|Sett6Count (Variables|/Game/views/saveGameObject.saveGameObject_C|Gett6Count _assave_game_object)))
      (:then_9
        (Variables|Default|Sett7Count (Variables|/Game/views/saveGameObject.saveGameObject_C|Gett7Count _assave_game_object)))
      (:then_10
        (Variables|Default|Sett8Count (Variables|/Game/views/saveGameObject.saveGameObject_C|Gett8Count _assave_game_object)))
      (:then_11
        (Variables|Default|Sett9Count (Variables|/Game/views/saveGameObject.saveGameObject_C|Gett9Count _assave_game_object)))
      (:then_12
        (Variables|Default|Sett10Count (Variables|/Game/views/saveGameObject.saveGameObject_C|Gett10Count _assave_game_object)))
      (:then_13
        (Variables|Default|SetclickIncrementValue (Variables|/Game/views/saveGameObject.saveGameObject_C|GetclickIncrementValue _assave_game_object))
        (return true)))
    (else
      (Development|PrintString "Slot doesn't exist" true true "(R=1.000000,G=0.000000,B=0.000000,A=1.000000)" 5.0))))